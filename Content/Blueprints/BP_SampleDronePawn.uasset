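; Sample drone pawn that manages first-person and third-person cameras and animates the rotors, starting in FPV.
; The toggle-view input swaps the active camera through SetCameraMode.
; Each tick, the active flight mode's tilt setting makes the FPV spring arm level, tilted or counter-rotated against pitch and roll, while the third-person arm follows only yaw.
; Four rotor components spin at a fixed rate, independent of throttle.
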(event Input|EnhancedActionEvents|EnhancedInputActionIA_ToggleView
  (params (ActionValue :type Boolean) (ElapsedSeconds :type Float%20%28double-precision%29) (TriggeredSeconds :type Float%20%28double-precision%29) (InputAction :type Input%20Action%20Object%20Reference :default "/DroneSimulator/Blueprints/IA_ToggleView.IA_ToggleView"))
  (if (Variables|Default|GetIs%20camera%20FPV)
    (CallFunction|SetCameraMode false)
    (else
      (CallFunction|SetCameraMode true))))

(event EventTick
  (params (DeltaSeconds :type Float%20%28single-precision%29))
  (bind _returnvalue (Transformation|GetActorRotation))
  (bind _returnvalue_2 (* DeltaSeconds 3.6e+02 8.0))
  (bind _springarm_fpv (Variables|Default|GetSpringArm_FPV))
  (bind _returnvalue_3 (Math|Rotator|MakeRotator 0.0 0.0 _returnvalue_2))
  (bind (_roll _pitch) (Math|Rotator|BreakRotator _returnvalue))
  (Utilities|FlowControl|Sequence
    (:then_0
      (switch Utilities|FlowControl|Switch|SwitchonECameraTiltMode (Class|FlightModeBase|GetCameraTiltMode (Class|DroneMovementComponent|GetActiveFlightMode (Variables|Default|Getmovement_component)))
        (:Zero
          (Transformation|SetRelativeRotation _springarm_fpv "0, 0, 0" false false))
        (:Tilted
          (Transformation|SetRelativeRotation _springarm_fpv "15.000000,0.000000,0.000000" false false))
        (:Stabilized
          (Transformation|SetRelativeRotation _springarm_fpv (Math|Rotator|MakeRotator (* _roll -1.0) (* _pitch -1.0) 0.0) false false))))
    (:then_1
      (Transformation|SetWorldRotation (Variables|Default|GetSpringArm_3P) (Math|Rotator|MakeRotator 0.0 0.0 (.Yaw (Math|Rotator|BreakRotator (Transformation|GetActorRotation)))) false false))
    (:then_2
      (Transformation|AddRelativeRotation (Variables|Default|GetMotorFL) _returnvalue_3 false false)
      (Transformation|AddRelativeRotation (Variables|Default|GetMotorFR) _returnvalue_3 false false)
      (Transformation|AddRelativeRotation (Variables|Default|GetMotorRL) _returnvalue_3 false false)
      (Transformation|AddRelativeRotation (Variables|Default|GetPropRR) _returnvalue_3 false false))))

(event EventBeginPlay
  (CallFunction|SetCameraMode true))

(fn ConstructionScript)

(fn SetCameraMode
  (params (New%20camera%20is%20FPV :type Boolean))
  (Components|Activation|SetActive (Variables|Default|GetCamera_3P) (not New%20camera%20is%20FPV) false)
  (Components|Activation|SetActive (Variables|Default|GetCamera_FPV) New%20camera%20is%20FPV false)
  (Variables|Default|SetIs%20camera%20FPV New%20camera%20is%20FPV))