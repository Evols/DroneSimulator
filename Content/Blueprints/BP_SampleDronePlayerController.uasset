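; Player controller for the sample drone that sets up the HUD and Enhanced Input mapping context on BeginPlay.
; Input actions open the calibration menu and toggle the pawn's DroneMovementComponent between race and stabilized flight modes.
; Restart unpossesses the current pawn without destroying it, then spawns and possesses a new drone using randomly picked PlayerStart transforms, falling back to the origin.
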(event Input|EnhancedActionEvents|EnhancedInputActionIA_ToggleCalibration
  (params (ActionValue :type Boolean) (ElapsedSeconds :type Float%20%28double-precision%29) (TriggeredSeconds :type Float%20%28double-precision%29) (InputAction :type Input%20Action%20Object%20Reference :default "/DroneSimulator/Blueprints/IA_ToggleCalibration.IA_ToggleCalibration"))
  (Class|DronePlayerController|ShowCalibrationMenu))

(event Input|EnhancedActionEvents|EnhancedInputActionIA_Mode
  (params (ActionValue :type Boolean) (ElapsedSeconds :type Float%20%28double-precision%29) (TriggeredSeconds :type Float%20%28double-precision%29) (InputAction :type Input%20Action%20Object%20Reference :default "/DroneSimulator/Blueprints/IA_Mode.IA_Mode"))
  (bind _returnvalue (Game|Player|GetPlayerPawn 0))
  (bind _returnvalue_2 (Actor|GetComponentbyClass _returnvalue "/Script/DroneSimulator.DroneMovementComponent"))
  (switch name (Class|DroneMovementComponent|GetActiveFlightModeName _returnvalue_2)
    (:race
      (Class|DroneMovementComponent|SetActiveFlightMode _returnvalue_2 "stabilized"))
    (:stabilized
      (Class|DroneMovementComponent|SetActiveFlightMode _returnvalue_2 "race"))))

(event Input|EnhancedActionEvents|EnhancedInputActionIA_Restart
  (params (ActionValue :type Boolean) (ElapsedSeconds :type Float%20%28double-precision%29) (TriggeredSeconds :type Float%20%28double-precision%29) (InputAction :type Input%20Action%20Object%20Reference :default "/DroneSimulator/Blueprints/IA_Restart.IA_Restart"))
  (Utilities|FlowControl|Sequence
    (:then_0
      (Pawn|UnPossess))
    (:then_1
      (bind _outactors (Actor|GetAllActorsOfClass "/Script/Engine.PlayerStart"))
      (bind _returnvalue (Game|SpawnActorfromClass "/DroneSimulator/Blueprints/BP_SampleDronePawn.BP_SampleDronePawn_C" (Math|Transform|MakeTransform (.Location (Math|Transform|BreakTransform (select (Utilities|IsValid (Utilities|Array|Get(acopy) _outactors (Math|Random|RandomInteger (Utilities|Array|Length _outactors)))) (Transformation|GetActorTransform (Utilities|Array|Get(acopy) _outactors (Math|Random|RandomInteger (Utilities|Array|Length _outactors)))) (Math|Transform|MakeTransform "0, 0, 0")))) (.Rotation (Math|Transform|BreakTransform (select (Utilities|IsValid (Utilities|Array|Get(acopy) _outactors (Math|Random|RandomInteger (Utilities|Array|Length _outactors)))) (Transformation|GetActorTransform (Utilities|Array|Get(acopy) _outactors (Math|Random|RandomInteger (Utilities|Array|Length _outactors)))) (Math|Transform|MakeTransform "0, 0, 0"))))) "Undefined" "MultiplyWithRoot" self 0))
      (Pawn|Possess _returnvalue))))

(event EventBeginPlay
  (Utilities|FlowControl|Sequence
    (:then_0
      (bind _returnvalue (UserInterface|CreateWidget "/DroneSimulator/UI/WB_HUD.WB_HUD_C"))
      (UserInterface|Viewport|AddtoPlayerScreen _returnvalue))
    (:then_1
      (Input|AddMappingContext (PlayerController|LocalPlayerSubsystems|GetEnhancedInputLocalPlayerSubsystem self) (Variables|Default|GetMapping%20context) 0 "(bIgnoreAllPressedKeysUntilRelease=True,bForceImmediately=False,bNotifyUserSettings=False)"))))

(fn ConstructionScript)